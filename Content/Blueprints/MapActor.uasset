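; MapActor is a map actor that sizes its base plane to the dimensions of a block-based map.
; UpdateMapSize scales the BasePlane1x1 component on X and Y by the map's width and height in blocks multiplied by the block width and height, leaving Z at one.
; The construction script and BeginPlay both call it, so the plane is sized on construction and again when play starts.
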(event EventBeginPlay
  (CallFunction|UpdateMapSize))

(event Collision|EventActorBeginOverlap
  (params (OtherActor :type Actor%20Object%20Reference)))

(event EventTick
  (params (DeltaSeconds :type Float%20%28single-precision%29)))

(fn ConstructionScript
  (CallFunction|UpdateMapSize))

(fn UpdateMapSize
  (Transformation|SetWorldScale3D (Variables|Default|Getbase_plane_1x1) (Math|Vector|MakeVector (Math|Conversions|ToFloat(Integer) (* (Variables|Default|Getwidth) (Variables|Default|GetblockWidth))) (Math|Conversions|ToFloat(Integer) (* (Variables|Default|Getheight) (Variables|Default|GetblockHeight))) 1.0)))