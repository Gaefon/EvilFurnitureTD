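; RTS player controller that handles edge-scroll camera movement and mouse box selection.
; On begin play it moves the controlled pawn to the center of the first MapActor's grid.
; Each tick, the cursor in the outer 10% of the viewport drives pawn movement input.
; SelectInput starts and ends selection on SimpleHUD, whose start point shifts by an empirical ratio of camera input to offset scrolling.
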(event EventBeginPlay
  (CallFunction|SetDefaultPlacement))

(event EventTick
  (params (DeltaSeconds :type Float%20%28single-precision%29))
  (bind _newparam (CallFunction|MoveCamerawithDeltaSec DeltaSeconds))
  (CallFunction|UpdateMouseSelection _newparam))

(event Input|ActionEvents|InputActionSelectInput
  (params (Key :type Key%20Structure))
  (bind (_locationx _locationy) (Game|Player|GetMousePosition))
  (bind _returnvalue (Math|Vector2D|MakeVector2D _locationx _locationy))
  (:Pressed
    (bind _assimple_hud (Utilities|Casting|CastToSimpleHUD (HUD|GetHUD)))
    (Variables|/Game/Blueprints/SimpleHUD.SimpleHUD_C|SetstartSelection _assimple_hud _returnvalue)
    (Variables|/Game/Blueprints/SimpleHUD.SimpleHUD_C|SetcurrentSelection _assimple_hud _returnvalue)
    (Variables|/Game/Blueprints/SimpleHUD.SimpleHUD_C|SetisSelecting _assimple_hud true))
  (:Released
    (bind _assimple_hud_2 (Utilities|Casting|CastToSimpleHUD (HUD|GetHUD)))
    (Variables|/Game/Blueprints/SimpleHUD.SimpleHUD_C|SetisSelecting _assimple_hud_2 false)))

(fn ConstructionScript)

(fn GetMovementVector
  (bind _returnvalue (Viewport|GetViewportSize))
  (bind (_locationx _locationy) (Game|Player|GetMousePosition))
  (bind (_x _y) (Math|Vector2D|BreakVector2D _returnvalue))
  (Utilities|FlowControl|Sequence
    (:then_0
      (LocalVariables|SetnewVector "(X=0.000000,Y=0.000000)"))
    (:then_1
      (if (< _locationx (* _x 0.1))
        (LocalVariables|SetnewVector (Math|Vector2D|MakeVector2D -1.0 (.y (LocalVariables|GetnewVector))))))
    (:then_2
      (if (> _locationx (* _x 0.9))
        (LocalVariables|SetnewVector (Math|Vector2D|MakeVector2D 1.0 (.y (LocalVariables|GetnewVector))))))
    (:then_3
      (if (< _locationy (* _y 0.1))
        (LocalVariables|SetnewVector (Math|Vector2D|MakeVector2D (.x (LocalVariables|GetnewVector)) 1.0))))
    (:then_4
      (if (> _locationy (* _y 0.9))
        (LocalVariables|SetnewVector (Math|Vector2D|MakeVector2D (.x (LocalVariables|GetnewVector)) -1.0))))
    (:then_5
      (return (LocalVariables|GetnewVector)))))

(fn MoveCamerawithDeltaSec
  (params (deltaSec :type Float%20%28single-precision%29))
  (bind _vectorout (CallFunction|GetMovementVector))
  (Pawn|Input|AddMovementInput (Pawn|GetControlledPawn) (Math|Vector|MakeVector (.y (* _vectorout (* deltaSec (Variables|Default|GetscrollSensivity)))) (.x (* _vectorout (* deltaSec (Variables|Default|GetscrollSensivity)))) 0.0) 1.0 false)
  (return (Math|Vector|MakeVector (.y (* _vectorout (* deltaSec (Variables|Default|GetscrollSensivity)))) (.x (* _vectorout (* deltaSec (Variables|Default|GetscrollSensivity)))) 0.0)))

(fn UpdateMouseSelection
  (params (CameraMovementInput :type Vector))
  (bind (_locationx _locationy) (Game|Player|GetMousePosition))
  (bind (_x _y) (Math|Vector|BreakVector CameraMovementInput))
  (bind _assimple_hud (Utilities|Casting|CastToSimpleHUD (HUD|GetHUD)))
  (if (Variables|/Game/Blueprints/SimpleHUD.SimpleHUD_C|GetisSelecting _assimple_hud)
    (Variables|/Game/Blueprints/SimpleHUD.SimpleHUD_C|SetcurrentSelection _assimple_hud (Math|Vector2D|MakeVector2D _locationx _locationy))
    (Variables|/Game/Blueprints/SimpleHUD.SimpleHUD_C|SetstartSelection _assimple_hud (- (Variables|/Game/Blueprints/SimpleHUD.SimpleHUD_C|GetstartSelection _assimple_hud) (Math|Vector2D|MakeVector2D (* _y 0.5) (* _x -0.5)))) ; Prends en compte le mouvement de la camera pour eviter d'avoir la selection qui scroll
  ))

(fn SetDefaultPlacement
  (bind _outactors (Actor|GetAllActorsOfClass "/Game/Blueprints/MapActor.MapActor_C"))
  (Transformation|SetActorLocationAndRotation (Pawn|GetControlledPawn) (Math|Vector|MakeVector (Math|Conversions|ToFloat(Integer) (/ (* (Variables|/Game/Blueprints/MapActor.MapActor_C|Getwidth (Utilities|Array|Get(acopy) _outactors)) (Variables|/Game/Blueprints/MapActor.MapActor_C|GetblockWidth (Utilities|Array|Get(acopy) _outactors))) 2)) (Math|Conversions|ToFloat(Integer) (/ (* (Variables|/Game/Blueprints/MapActor.MapActor_C|Getheight (Utilities|Array|Get(acopy) _outactors)) (Variables|/Game/Blueprints/MapActor.MapActor_C|GetblockHeight (Utilities|Array|Get(acopy) _outactors))) 2)) (.z (Variables|Default|GetinitialLocation)))))