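; MyRobot is an input-driven robot Blueprint with tank-style movement.
; The MoveUpDown axis moves it along its facing on the horizontal plane, using cosine and sine of yaw scaled by MoveSpeed.
; The MoveLeftRight axis turns it in yaw by RotationSpeed.
; Both set the transform directly without delta-time scaling, and movement does not sweep for collision.
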(event Input|AxisEvents|InputAxisMoveUpDown
  (params (AxisValue :type Float%20%28single-precision%29))
  (bind _returnvalue (Transformation|GetActorRotation))
  (bind _movespeed (Variables|Bot|GetMoveSpeed))
  (bind _yaw (Math|Rotator|BreakRotator _returnvalue))
  (bind _returnvalue_2 (* AxisValue _movespeed))
  (Transformation|SetActorLocation (+ (Transformation|GetActorLocation) (Math|Vector|MakeVector (* _returnvalue_2 (Math|Trig|Cos(Degrees) _yaw)) (* _returnvalue_2 (Math|Trig|Sin(Degrees) _yaw)) 0.0)) false false))

(event Input|AxisEvents|InputAxisMoveLeftRight
  (params (AxisValue :type Float%20%28single-precision%29))
  (Transformation|SetActorRotation (Math|Rotator|CombineRotators (Transformation|GetActorRotation) (Math|Rotator|MakeRotator 0.0 0.0 (* AxisValue (Variables|Bot|GetRotationSpeed))))))

(fn ConstructionScript)