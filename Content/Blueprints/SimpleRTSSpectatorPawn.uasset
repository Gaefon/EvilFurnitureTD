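; SimpleRTSSpectatorPawn is a spectator pawn that provides an RTS camera with smooth zoom and map bounds.
; ZoomIn and ZoomOut inputs step a clamped target zoom, which Tick interpolates into the SpringArm length.
; Each tick it also looks up the first MapActor and clamps the spring arm's X to map height and Y to map width, using Min/Max instead of branches, then moves the pawn there.
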(event EventBeginPlay
  (Variables|/Script/Engine.SpringArmComponent|SetTargetArmLength (Variables|Default|GetSpringArm) (Variables|Default|GetcurrentZoom)))

(event Collision|EventActorBeginOverlap
  (params (OtherActor :type Actor%20Object%20Reference)))

(event EventTick
  (params (DeltaSeconds :type Float%20%28single-precision%29))
  (CallFunction|UpdateCamZoom DeltaSeconds)
  (CallFunction|CheckPositioninMap))

(event Input|ActionEvents|InputActionZoomIn
  (params (Key :type Key%20Structure))
  (:Pressed
    (Variables|Default|SetdesiredCamZoom (Math|Float|Clamp(Float) (- (Variables|Default|GetdesiredCamZoom) (Variables|Default|GetzoomSensivity)) (Variables|Default|GetminZoom) (Variables|Default|GetmaxZoom)))))

(event Input|ActionEvents|InputActionZoomOut
  (params (Key :type Key%20Structure))
  (:Pressed
    (Variables|Default|SetdesiredCamZoom (Math|Float|Clamp(Float) (+ (Variables|Default|GetdesiredCamZoom) (Variables|Default|GetzoomSensivity)) (Variables|Default|GetminZoom) (Variables|Default|GetmaxZoom)))))

(fn ConstructionScript)

(fn UpdateCamZoom
  (params (deltaTime :type Float%20%28single-precision%29))
  (bind _desiredcamzoom (Variables|Default|GetdesiredCamZoom))
  (if (not (== (Variables|Default|GetcurrentZoom) _desiredcamzoom))
    (bind _output_get (Variables|Default|SetcurrentZoom (Math|Interpolation|FInterpTo (Variables|Default|GetcurrentZoom) _desiredcamzoom deltaTime (Variables|Default|GetzoomSpeed))))
    (Variables|/Script/Engine.SpringArmComponent|SetTargetArmLength (Variables|Default|GetSpringArm) _output_get)))

(fn CheckPositioninMap
  (bind _springarm (Variables|Default|GetSpringArm))
  (bind _returnvalue (Transformation|GetWorldLocation _springarm))
  (bind _outactors (Actor|GetAllActorsOfClass "/Game/Blueprints/MapActor.MapActor_C"))
  (Utilities|FlowControl|Sequence
    (:then_0
      (bind _real_height (Default|GetRealMapHeight (Utilities|Array|Get(acopy) _outactors))))
    (:then_1
      (bind _real_width (Default|GetRealMapWidth (Utilities|Array|Get(acopy) _outactors))))
    (:then_2
      (Transformation|SetActorLocation (Math|Vector|MakeVector (Math|Float|Min(Float) (Math|Float|Max(Float) (.x _returnvalue) 0.0) (Math|Conversions|ToFloat(Integer) _real_height)) (Math|Float|Min(Float) (Math|Float|Max(Float) (.y _returnvalue) 0.0) (Math|Conversions|ToFloat(Integer) _real_width)) (.z _returnvalue)) false false))))