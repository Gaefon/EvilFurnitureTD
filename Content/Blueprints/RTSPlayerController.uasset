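; RTS player controller that moves the camera pawn and holds the selected pawns.
; Tick runs a camera state machine: PanCamera drags the view via cursor ground-trace deltas, while the cursor in the outer 10% of the viewport scrolls it away from screen center.
; Tick also accumulates input-hold and move-click timers, notifying the HUD while input is held; the flags driving both are not set in this graph.
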(event Custom|UpdateSelection
  (if (Variables|Default|GetIsHoldingInput)
    (Variables|Default|SetInputHoldingTime (+ (Variables|Default|GetInputHoldingTime) (Variables|Default|GetDeltaTime)))
    (Class|InputInterface|OnInputHold(Message) (HUD|GetHUD))))

(event Custom|UpdateClickToMove
  (if (Variables|Default|GetWantToMove)
    (Variables|Default|SetMoveClickTime (+ (Variables|Default|GetMoveClickTime) (Variables|Default|GetDeltaTime)))))

(event EventBeginPlay)

(event EventTick
  (params (DeltaSeconds :type Float%20%28single-precision%29))
  (Variables|Default|SetDeltaTime DeltaSeconds)
  (CallFunction|UpdateCamera)
  (CallFunction|UpdateSelection)
  (CallFunction|UpdateClicktoMove))

(event Input|ActionEvents|InputActionPanCamera
  (params (Key :type Key%20Structure))
  (:Pressed
    (CallFunction|OnSwipeStarted)
    (Variables|Default|SetCurrentInputState "NewEnumerator2")
    (Variables|Default|SetIsCameraScrolling true))
  (:Released
    (CallFunction|OnSwipeEnded)
    (Variables|Default|SetCurrentInputState "NewEnumerator0")))

(fn ConstructionScript)

(fn OnSwipeStarted
  (Variables|Default|SetStartSwipeCoords (.Location (Collision|BreakHitResult (.HitResult (Game|Player|GetHitResultUnderCursorbyChannel "TraceTypeQuery3" true))))))

(fn OnSwipeUpdate
  (LocalVariables|SetLocal%20New%20Swipe%20Coords (.Location (Collision|BreakHitResult (.HitResult (Game|Player|GetHitResultUnderCursorbyChannel "TraceTypeQuery3" true)))))
  (bind _output_get (LocalVariables|SetLocal%20Delta (Math|Vector|MakeVector (.X (Math|Vector|BreakVector (- (Variables|Default|GetStartSwipeCoords) (LocalVariables|GetLocal%20New%20Swipe%20Coords)))) (.Y (Math|Vector|BreakVector (- (Variables|Default|GetStartSwipeCoords) (LocalVariables|GetLocal%20New%20Swipe%20Coords)))) 0.0)))
  (return _output_get))

(fn SetSelectedPawns
  (params (SelectedPawns :type Actor%20Object%20Reference))
  (Variables|Default|SetSelectedPawns SelectedPawns))

(fn GetScrollDirection
  (bind _returnvalue (Viewport|GetViewportSize))
  (bind (_locationx _locationy) (Game|Player|GetMousePosition))
  (bind _returnvalue_2 (Math|Vector2D|MakeVector2D _locationx _locationy))
  (bind _returnvalue_3 (/ _returnvalue 2.0))
  (bind _returnvalue_4 (- _returnvalue_2 _returnvalue_3))
  (bind _returnvalue_5 (Math|Conversions|ToVector(Vector2D) _returnvalue_4))
  (bind _returnvalue_6 (* _returnvalue_5 1.0))
  (bind _returnvalue_7 (Math|Vector|ClampVectorSize _returnvalue_6 0.2 1.0))
  (bind (_x _y) (Math|Vector|BreakVector _returnvalue_7))
  (return (Math|Vector|MakeVector _y (* _x -1.0) 0.0)))

(fn UpdateCamera
  (bind _returnvalue (Pawn|GetControlledPawn))
  (switch Utilities|FlowControl|Switch|SwitchonEInputType (Variables|Default|GetCurrentInputState)
    (:NewEnumerator0
      (bind _drag (CallFunction|IsScrolling :!label _label))
      (if (Utilities|Enum|NotEqual(Enum) _drag "NewEnumerator0")
        (bind _direction (CallFunction|GetScrollDirection))
        (Pawn|Input|AddMovementInput (Pawn|GetControlledPawn) _direction 1.0 false)
        (Variables|Default|SetCurrentInputState "NewEnumerator3")))
    (:NewEnumerator2
      (if (Variables|Default|GetIsCameraScrolling)
        (bind _newparam (CallFunction|OnSwipeUpdate))
        (Transformation|SetActorLocation _returnvalue (+ _newparam (Transformation|GetActorLocation _returnvalue)) false false)))
    (:NewEnumerator3
      (goto _label))))

(fn IsScrolling
  (bind (_locationx _locationy) (Game|Player|GetMousePosition))
  (bind _returnvalue (Viewport|GetViewportSize))
  (bind (_locationx_2 _locationy_2) (Game|Player|GetMousePosition))
  (bind (_locationx_3 _locationy_3) (Game|Player|GetMousePosition))
  (bind _returnvalue_2 (Viewport|GetViewportSize))
  (bind (_x _y) (Math|Vector2D|BreakVector2D _returnvalue))
  (bind (_x_2 _y_2) (Math|Vector2D|BreakVector2D _returnvalue_2))
  (bind _returnvalue_3 (* _x_2 0.1))
  (bind _returnvalue_4 (* _y_2 0.1))
  (bind _returnvalue_5 (< _locationy_2 _returnvalue_4))
  (bind _returnvalue_6 (< _locationx_2 _returnvalue_3))
  (Utilities|FlowControl|Sequence
    (:then_0
      (if _returnvalue_6
        (LocalVariables|SetLocalDrag "NewEnumerator1")))
    (:then_1
      (if (and (not _returnvalue_6) (> _locationx_3 (* _x 0.9)))
        (LocalVariables|SetLocalDrag "NewEnumerator2")))
    (:then_2
      (if _returnvalue_5
        (LocalVariables|SetLocalDrag "NewEnumerator3")))
    (:then_3
      (if (and (not _returnvalue_5) (> _locationy_3 (* _y 0.9)))
        (LocalVariables|SetLocalDrag "NewEnumerator4")))
    (:then_4
      (if (and (== _locationx 0.0) (== 0.0 _locationy))
        (LocalVariables|SetLocalDrag "NewEnumerator0")))
    (:then_5
      (return (LocalVariables|GetLocalDrag)))))

(fn OnSwipeEnded
  (Variables|Default|SetEndSwipeCoords (.Location (Collision|BreakHitResult (.HitResult (Game|Player|GetHitResultUnderCursorbyChannel "TraceTypeQuery3" true)))))
  (Variables|Default|SetStartSwipeCoords "0, 0, 0"))