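; RTS spectator pawn Blueprint that provides smooth camera zoom through its spring arm.
; ZoomIn and ZoomOut inputs step a desired arm length up and down respectively, clamped between minimum and maximum limits.
; Tick interpolates the current zoom toward that target with FInterpTo and applies it to the spring arm, which BeginPlay initializes to the desired value.
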(event Custom|SetDefaultCamSettings
  (bind _output_get (Variables|Default|SetCurrentCamZoom (Variables|Default|GetDesiredCamZoom)))
  (Variables|/Script/Engine.SpringArmComponent|SetTargetArmLength (Variables|Default|GetSpringArm) _output_get))

(event Custom|UpdateCamZoom
  (if (not (== (Variables|Default|GetDesiredCamZoom) (Variables|Default|GetCurrentCamZoom)))
    (Variables|Default|SetCurrentCamZoom (Math|Interpolation|FInterpTo (Variables|Default|GetCurrentCamZoom) (Variables|Default|GetDesiredCamZoom) (Variables|Default|GetDeltaTime) (Variables|Default|GetCamZoomSpeed)))
    (Variables|/Script/Engine.SpringArmComponent|SetTargetArmLength (Variables|Default|GetSpringArm) (Variables|Default|GetCurrentCamZoom))))

(event EventBeginPlay
  (CallFunction|SetDefaultCamSettings))

(event Collision|EventActorBeginOverlap
  (params (OtherActor :type Actor%20Object%20Reference)))

(event EventTick
  (params (DeltaSeconds :type Float%20%28single-precision%29))
  (Variables|Default|SetDeltaTime DeltaSeconds)
  (CallFunction|UpdateCamZoom))

(event Input|ActionEvents|InputActionZoomIn
  (params (Key :type Key%20Structure))
  (:Pressed
    (Variables|Default|SetDesiredCamZoom (Math|Float|Clamp(Float) (+ (Variables|Default|GetDesiredCamZoom) 5e+01) (Variables|Default|GetMinCamZoom) (Variables|Default|GetMaxCamZoom)))))

(event Input|ActionEvents|InputActionZoomOut
  (params (Key :type Key%20Structure))
  (:Pressed
    (Variables|Default|SetDesiredCamZoom (Math|Float|Clamp(Float) (+ (Variables|Default|GetDesiredCamZoom) -5e+01) (Variables|Default|GetMinCamZoom) (Variables|Default|GetMaxCamZoom)))))

(fn ConstructionScript)