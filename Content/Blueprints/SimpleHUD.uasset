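; HUD that draws a bottom-right minimap and a translucent drag-selection rectangle every frame in DrawHUD.
; The minimap fits the first MapActor's bounds into its container with a uniform min-ratio scale and centering margins, looking the actor up on each draw.
; A cross marks the controlled pawn, mapping world Y to horizontal and inverted world X to vertical.
; The selection rectangle reads state variables that this graph never sets.
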(event EventBeginPlay)

(event Collision|EventActorBeginOverlap
  (params (OtherActor :type Actor%20Object%20Reference)))

(event EventTick
  (params (DeltaSeconds :type Float%20%28single-precision%29)))

(event EventDrawHUD
  (params (SizeX :type Integer) (SizeY :type Integer))
  (CallFunction|DrawMiniMap SizeX SizeY)
  (CallFunction|DrawRectSelection))

(fn ConstructionScript)

(fn DrawRectSelection
  (bind _startselection (Variables|Default|GetstartSelection))
  (bind _startselection_2 (Variables|Default|GetstartSelection))
  (bind _currentselection (Variables|Default|GetcurrentSelection))
  (bind _returnvalue (- _currentselection _startselection_2))
  (if (Variables|Default|GetisSelecting)
    (HUD|DrawRect "(R=0.000000,G=0.000000,B=0.000000,A=0.400000)" (.x _startselection) (.y _startselection) (.x _returnvalue) (.y _returnvalue))))

(fn DrawMiniMap
  (params (SizeX :type Integer) (SizeY :type Integer))
  (bind _minimapcontainerheight (Variables|Default|GetminimapContainerHeight))
  (bind _minimapcontainerwidth (Variables|Default|GetminimapContainerWidth))
  (HUD|DrawRect "(R=0,G=0,B=0,A=1)" (Math|Conversions|ToFloat(Integer) (- SizeX _minimapcontainerwidth)) (Math|Conversions|ToFloat(Integer) (- SizeY _minimapcontainerheight)) (Math|Conversions|ToFloat(Integer) _minimapcontainerwidth) (Math|Conversions|ToFloat(Integer) _minimapcontainerheight))
  (CallFunction|DrawMapBounds SizeX SizeY)
  (CallFunction|DrawMiniMapPosition SizeX SizeY))

(fn DrawMiniMapPosition
  (params (width :type Integer) (height :type Integer))
  (bind _returnvalue (Game|GetPlayerController 0))
  (bind _cross_size (LocalVariables|Getcross_size))
  (bind _cross_size_2 (LocalVariables|Getcross_size))
  (bind _returnvalue_2 (Pawn|GetControlledPawn _returnvalue))
  (bind _returnvalue_3 (Transformation|GetActorLocation _returnvalue_2))
  (Utilities|FlowControl|Sequence
    (:then_0
      (bind _outactors (Actor|GetAllActorsOfClass "/Game/Blueprints/MapActor.MapActor_C")))
    (:then_1
      (bind _ratio (CallFunction|GetMapBlockResizeRatio (Utilities|Array|Get(acopy) _outactors))))
    (:then_2
      ;[1 1 1] calculate the position ratio on the map and calculate the positon on the minimap
      (bind _real_height (Default|GetRealMapHeight (Utilities|Array|Get(acopy) _outactors))))
    (:then_3
      (bind _real_width (Default|GetRealMapWidth (Utilities|Array|Get(acopy) _outactors))))
    (:then_4
      ;[1 1 1] calculate the position on the HUD
      (bind (_x _y) (CallFunction|GetMapMargins (Utilities|Array|Get(acopy) _outactors))))
    (:then_5
      ;[1 1 1] Draw cross on the position
      (Class|HUD|DrawLine (- (+ _x (Math|Conversions|ToFloat(Integer) (- width (Variables|Default|GetminimapContainerWidth))) (* _ratio (* (Variables|/Game/Blueprints/MapActor.MapActor_C|Getwidth (Utilities|Array|Get(acopy) _outactors)) (/ (.y _returnvalue_3) (Math|Conversions|ToFloat(Integer) _real_width))))) _cross_size_2) (+ _y (Math|Conversions|ToFloat(Integer) (- height (Variables|Default|GetminimapContainerHeight))) (* _ratio (* (Variables|/Game/Blueprints/MapActor.MapActor_C|Getheight (Utilities|Array|Get(acopy) _outactors)) (- 1.0 (/ (.x _returnvalue_3) (Math|Conversions|ToFloat(Integer) _real_height)))))) (+ (+ _x (Math|Conversions|ToFloat(Integer) (- width (Variables|Default|GetminimapContainerWidth))) (* _ratio (* (Variables|/Game/Blueprints/MapActor.MapActor_C|Getwidth (Utilities|Array|Get(acopy) _outactors)) (/ (.y _returnvalue_3) (Math|Conversions|ToFloat(Integer) _real_width))))) _cross_size_2) (+ _y (Math|Conversions|ToFloat(Integer) (- height (Variables|Default|GetminimapContainerHeight))) (* _ratio (* (Variables|/Game/Blueprints/MapActor.MapActor_C|Getheight (Utilities|Array|Get(acopy) _outactors)) (- 1.0 (/ (.x _returnvalue_3) (Math|Conversions|ToFloat(Integer) _real_height)))))) "(R=1.000000,G=1.000000,B=1.000000,A=1.000000)" 1.0))
    (:then_6
      (Class|HUD|DrawLine (+ _x (Math|Conversions|ToFloat(Integer) (- width (Variables|Default|GetminimapContainerWidth))) (* _ratio (* (Variables|/Game/Blueprints/MapActor.MapActor_C|Getwidth (Utilities|Array|Get(acopy) _outactors)) (/ (.y _returnvalue_3) (Math|Conversions|ToFloat(Integer) _real_width))))) (- (+ _y (Math|Conversions|ToFloat(Integer) (- height (Variables|Default|GetminimapContainerHeight))) (* _ratio (* (Variables|/Game/Blueprints/MapActor.MapActor_C|Getheight (Utilities|Array|Get(acopy) _outactors)) (- 1.0 (/ (.x _returnvalue_3) (Math|Conversions|ToFloat(Integer) _real_height)))))) _cross_size) (+ _x (Math|Conversions|ToFloat(Integer) (- width (Variables|Default|GetminimapContainerWidth))) (* _ratio (* (Variables|/Game/Blueprints/MapActor.MapActor_C|Getwidth (Utilities|Array|Get(acopy) _outactors)) (/ (.y _returnvalue_3) (Math|Conversions|ToFloat(Integer) _real_width))))) (+ (+ _y (Math|Conversions|ToFloat(Integer) (- height (Variables|Default|GetminimapContainerHeight))) (* _ratio (* (Variables|/Game/Blueprints/MapActor.MapActor_C|Getheight (Utilities|Array|Get(acopy) _outactors)) (- 1.0 (/ (.x _returnvalue_3) (Math|Conversions|ToFloat(Integer) _real_height)))))) _cross_size) "(R=1.000000,G=1.000000,B=1.000000,A=1.000000)" 1.0))))

(fn DrawMapBounds
  (params (width :type Integer) (height :type Integer))
  (bind _outactors (Actor|GetAllActorsOfClass "/Game/Blueprints/MapActor.MapActor_C"))
  (Utilities|FlowControl|Sequence
    (:then_0
      (bind _ratio (CallFunction|GetMapBlockResizeRatio (Utilities|Array|Get(acopy) _outactors))))
    (:then_1
      (bind (_x _y) (CallFunction|GetMapMargins (Utilities|Array|Get(acopy) _outactors))))
    (:then_2
      (HUD|DrawRect "(R=0.200415,G=0.166016,B=1.000000,A=1.000000)" (+ _x (Math|Conversions|ToFloat(Integer) (- width (Variables|Default|GetminimapContainerWidth)))) (+ _y (Math|Conversions|ToFloat(Integer) (- height (Variables|Default|GetminimapContainerHeight)))) (* (Variables|/Game/Blueprints/MapActor.MapActor_C|Getwidth (Utilities|Array|Get(acopy) _outactors)) _ratio) (* (Variables|/Game/Blueprints/MapActor.MapActor_C|Getheight (Utilities|Array|Get(acopy) _outactors)) _ratio)))))

(fn GetMapBlockResizeRatio
  (params (map :type Map%20Actor%20Object%20Reference))
  (return (Math|Float|Min(Float) (/ (Math|Conversions|ToFloat(Integer) (Variables|Default|GetminimapContainerWidth)) (Math|Conversions|ToFloat(Integer) (Variables|/Game/Blueprints/MapActor.MapActor_C|Getwidth map))) (/ (Math|Conversions|ToFloat(Integer) (Variables|Default|GetminimapContainerHeight)) (Math|Conversions|ToFloat(Integer) (Variables|/Game/Blueprints/MapActor.MapActor_C|Getheight map))))))

(fn GetMapMargins
  (params (map :type Map%20Actor%20Object%20Reference))
  (bind _ratio (CallFunction|GetMapBlockResizeRatio map))
  (return (/ (- (Math|Conversions|ToFloat(Integer) (Variables|Default|GetminimapContainerWidth)) (* (Variables|/Game/Blueprints/MapActor.MapActor_C|Getwidth map) _ratio)) 2.0) (/ (- (Math|Conversions|ToFloat(Integer) (Variables|Default|GetminimapContainerHeight)) (* (Variables|/Game/Blueprints/MapActor.MapActor_C|Getheight map) _ratio)) 2.0)))